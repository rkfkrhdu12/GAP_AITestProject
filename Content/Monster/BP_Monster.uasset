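; BP_Monster is an AI-controlled enemy character with simple health and an Idle, Hit and Dead state machine.
; Hit takes one health point regardless of damage, entering Hit or Dead and recording the hit direction.
; Tick runs the Hit state once, disabling movement for half a direction-based montage before returning to Idle.
; Sword overlaps flag player contact, and GetCurSpeed zeroes speed when hit or dead.
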(event `self.ReceiveBeginPlay`
  (bind _asbp_monster_ai (cast `/Game/Monster/BP_MonsterAI` (`self.GetController`)))
  (set `self.CurController` _asbp_monster_ai))

(event `self.ReceiveTick`
  (params (DeltaSeconds :type "Float (single-precision)"))
  (bind _charactermovement (`self.CharacterMovement`))
  (switch `/Game/Monster/eMonsterState` (`self.CurState`)
    (:`NewEnumerator3`
      (if (`self.bStateEnable`)
        (set `self.bStateEnable` false)
        (set `self.CurAnimMontage` (`|GetArrayItem` (`self.AnimMontageHit`) (`KismetMathLibrary.Conv_BoolToInt` (`self.bHitForward`))))
        (`CharacterMovementComponent.DisableMovement` _charactermovement)
        (bind _returnvalue (`self.PlayAnimMontage` (`self.CurAnimMontage`)))
        (`KismetSystemLibrary.Delay` (* _returnvalue 0.5))
        (`self.StopAnimMontage` (`self.CurAnimMontage`))
        (set `self.CurState` "NewEnumerator0")
        (`CharacterMovementComponent.SetMovementMode` _charactermovement "MOVE_Walking" 0)))))

(event `self.Sword.OnComponentBeginOverlap`
  (params (OverlappedComponent :type "PrimitiveComponent Object Reference") (OtherActor :type "Actor Object Reference") (OtherComp :type "PrimitiveComponent Object Reference") (OtherBodyIndex :type Integer) (bFromSweep :type Boolean) (SweepResult :type "HitResult Structure (by ref)"))
  (cast `/Game/ThirdPersonCPP/ThirdPersonCharacter` OtherActor)
  (set `self.bOverlapPlayer` true))

(event `self.Sword.OnComponentEndOverlap`
  (params (OverlappedComponent :type "PrimitiveComponent Object Reference") (OtherActor :type "Actor Object Reference") (OtherComp :type "PrimitiveComponent Object Reference") (OtherBodyIndex :type Integer))
  (cast `/Game/ThirdPersonCPP/ThirdPersonCharacter` OtherActor)
  (set `self.bOverlapPlayer` false))

(fn `GetCurSpeed`
  (returns (CurSpeed :type "Float (double-precision)"))
  (locals (bCheckDirection :type Boolean) (bForward :type Boolean))
  (`|ExecutionSequence`
    (:`then_0`
      (switch `/Game/Monster/eMonsterState` (`self.CurState`)
        (:`NewEnumerator0`
          (`/Game/Monster/BP_MonsterAI.GetCurSpeed` (`self.CurController`)))
        (:`NewEnumerator5`
          (set `self.CurSpeed` 0.0 :!label _label))
        (:`NewEnumerator3`
          (goto _label))))
    (:`then_1`
      (return (`self.CurSpeed`)))))

(fn `Hit`
  (params (Damage :type "Float (double-precision)") (AttackActor :type "Actor Object Reference"))
  (returns (bSuccess :type Boolean))
  (set `self.bHitForward` (>= (`KismetMathLibrary.Dot_VectorVector` (- (`KismetMathLibrary.Normal` (`self.K2_GetActorLocation` AttackActor)) (`KismetMathLibrary.Normal` (`self.K2_GetActorLocation`))) (`self.GetActorForwardVector`)) 0.0))
  (bind _result (`/Engine/EditorBlueprintResources/StandardMacros.DecrementInt` (stale _output_get))
    (:`  `
      (bind _output_get (set `self.CurHealthPoint` _result))
      (if (> _output_get 0)
        (set `self.CurState` "NewEnumerator3")
        (set `self.bStateEnable` true)
        (return true)
        (else
          (set `self.CurState` "NewEnumerator5")
          (set `self.bDeath` true))))))

(fn `UserConstructionScript`)