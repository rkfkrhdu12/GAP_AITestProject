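; AI controller for BP_Monster that runs BT_Monster and chooses the monster's behavior: look at, attack, runaway or hide.
; Tick copies monster state, updates the behavior and writes it to the blackboard, pausing when the state changes.
; When idle it draws randomly from an enabled list; per-behavior delay macros re-add entries after cooldown.
; UpdateLookAt is an empty stub, and Runaway and Hide end immediately on update.
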(event `EndBehavior`
  (set `self.CurBehavior` "NewEnumerator4")
  (`self.UpdateCoolDown`))

(event `UpdateCoolDown`
  (bind _enumvalue (foreach `/Game/Monster/eMonsterBehavior` false)
    (:`LoopBody`
      (switch `/Game/Monster/eMonsterBehavior` _enumvalue
        (:`NewEnumerator0`
          (bind _returnvalue (== (`KismetArrayLibrary.Array_Find` (`self.BehaviorEnableList`) _enumvalue) -1))
          (if _returnvalue
            (`self.LookAtCoolDown`)))
        (:`NewEnumerator1`
          (if _returnvalue
            (`self.AttackCoolDown`)))
        (:`NewEnumerator2`
          (if _returnvalue
            (`self.RunawayCoolDown`)))
        (:`NewEnumerator3`
          (if _returnvalue
            (`self.HideCoolDown`)))))))

(event `self.ReceiveBeginPlay`
  (bind _asbp_monster (cast `/Game/Monster/BP_Monster` (`self.K2_GetPawn`)))
  (set `self.CurMonster` _asbp_monster)
  (`self.RunBehaviorTree` "/Game/Monster/BT_Monster.BT_Monster"))

(event `self.ReceiveTick`
  (params (DeltaSeconds :type "Float (single-precision)"))
  (bind _curmonster (`self.CurMonster`))
  (`/Engine/EditorBlueprintResources/StandardMacros.IsValid` _curmonster
    (:`Is Valid`
      (`|ExecutionSequence`
        (:`then_0`
          (set `self.Monster_CurState` (`/Game/Monster/BP_Monster.CurState` _curmonster)))
        (:`then_1`
          (if (`|EnumInequality` (`self.CurBehavior`) "NewEnumerator5")
            (`self.UpdateBehavior`)))
        (:`then_2`
          (`BlackboardComponent.SetValueAsEnum` (`self.Blackboard`) (`self.BB_CurBehaviorKeyName`) (`self.CurBehavior`)))))))

(fn `BehaviorPause`
  (if (`|EnumInequality` (`self.CurBehavior`) "NewEnumerator6")
    (set `self.PrevBehavior` (`self.CurBehavior`))
    (set `self.CurBehavior` "NewEnumerator6")
    (`NavMovementComponent.StopActiveMovement` (`Character.CharacterMovement` (`self.CurMonster`)))
    (elif (`|EnumEquality` (`self.Monster_CurState`) "NewEnumerator0")
      (set `self.CurBehavior` (`self.PrevBehavior`)))))

(fn `GetBehavior`
  (returns (NewBehavior :type "/Game/Monster/eMonsterBehavior Enum"))
  (bind _behaviorenablelist (`self.BehaviorEnableList`))
  (if (and (`|EnumEquality` (`self.CurBehavior`) "NewEnumerator4") (!= (`KismetArrayLibrary.Array_Length` (`self.BehaviorEnableList`)) 0))
    (bind _output_get (set `self.CurBehavior` (`|GetArrayItem` _behaviorenablelist (`KismetMathLibrary.RandomInteger` (`KismetArrayLibrary.Array_Length` _behaviorenablelist)))))
    (`KismetArrayLibrary.Array_RemoveItem` _behaviorenablelist _output_get)
    (return _output_get)))

(fn `GetCurSpeed`
  (bind _curmonster (`self.CurMonster`))
  (bind _returnvalue (`SceneComponent.GetForwardVector` (`Character.Mesh` _curmonster)))
  (if (`|EnumInequality` (`self.CurBehavior`) "NewEnumerator4")
    (`|ExecutionSequence`
      (:`then_0`
        (if (`KismetMathLibrary.NearlyEqual_FloatFloat` (`/Game/Monster/BP_Monster.CurSpeed` (`self.CurMonster`)) 0.0 0.1)
          (if (`self.bMoveDirectionUpdate`)
            (set `self.bMoveDirectionUpdate` false)
            (set `self.bMoveForward` (<= (`KismetMathLibrary.Vector_Distance` (`self.GetVelocity` _curmonster) _returnvalue) (`KismetMathLibrary.Vector_Distance` _returnvalue (* (`self.GetVelocity` _curmonster) -1)))))
          (else
            (set `self.bMoveDirectionUpdate` true))))
      (:`then_1`
        (set `/Game/Monster/BP_Monster.CurSpeed` (* (`KismetMathLibrary.SelectInt` 1 -1 (`self.bMoveForward`)) (`KismetMathLibrary.VSize` (`self.GetVelocity` (`self.CurMonster`)))) (`self.CurMonster`))))))

(fn `InitBehavior`
  (params (NewBehavior :type "/Game/Monster/eMonsterBehavior Enum" :default "NewEnumerator4"))
  (`|ExecutionSequence`
    (:`then_0`
      (switch `/Game/Monster/eMonsterBehavior` NewBehavior
        (:`NewEnumerator0`
          (`self.InitLookAt`))))
    (:`then_1`
      (set `self.CurBehavior` NewBehavior)
      (return))))

(fn `InitLookAt`
  (locals (LookAtTime :type "Float (double-precision)" :default 3.0))
  (bind _curmonster (`self.CurMonster`))
  (bind _returnvalue (`self.K2_GetActorLocation` _curmonster))
  (bind _returnvalue_2 (* (`SceneComponent.GetRightVector` (`Actor.RootComponent` _curmonster)) (* (`CharacterMovementComponent.MaxWalkSpeed` (`Character.CharacterMovement` _curmonster)) (`local.LookAtTime`))))
  (set `self.LookAtAlpha` 0.0)
  (`self.UpdateLookAt`)
  (if (`KismetMathLibrary.RandomBool`)
    (set `/Game/Monster/BP_Monster.MoveLocation` (+ _returnvalue_2 _returnvalue) (`self.CurMonster`))
    (set `self.bLookAtRight` true)
    (else
      (set `/Game/Monster/BP_Monster.MoveLocation` (+ (* _returnvalue_2 -1) _returnvalue) (`self.CurMonster`))
      (set `self.bLookAtRight` false))))

(fn `UpdateBehavior`
  (if (`|EnumEquality` (`self.Monster_CurState`) "NewEnumerator0")
    (switch `/Game/Monster/eMonsterBehavior` (`self.CurBehavior`)
      (:`NewEnumerator4`
        (bind _newbehavior (`self.GetBehavior`))
        (`self.InitBehavior` _newbehavior))
      (:`NewEnumerator0`
        (`self.UpdateLookAt`))
      (:`NewEnumerator2`
        (`self.EndBehavior` :!label _label))
      (:`NewEnumerator3`
        (goto _label)))
    (else
      (`self.BehaviorPause`))))

(fn `UpdateLookAt`)

(fn `UserConstructionScript`)